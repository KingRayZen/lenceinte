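; Weather manager actor that runs a day-night cycle, driving the directional light, sky sphere and HUD clock.
; At start it finds the sun, sky and fog actors, records the sun's intensity and converts the start time into scaled elapsed seconds.
; Each tick it advances time, rotates the sun, fades its intensity by sunrise and sunset hours, and sends the current time to the player's HUD.
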(event EventBeginPlay
  (Utilities|FlowControl|Sequence
    (:then_0
      (CallFunction|GetSunandSky))
    (:then_1
      (CallFunction|SetSunIntensity))
    (:then_2
      (CallFunction|SetElapsedTime))))

(event EventTick
  (params (DeltaSeconds :type Float%20%28single-precision%29))
  (Utilities|FlowControl|Sequence
    (:then_0
      (CallFunction|UpdateElapsedTime))
    (:then_1
      (CallFunction|UpdateSunPosition))
    (:then_2
      (CallFunction|SetHUDRef))
    (:then_3
      (CallFunction|FadeSun))
    (:then_4
      (CallFunction|UpdateCurrentTime))))

(fn ConstructionScript
  (Variables|Default|SetSecondsPerDay (* (Variables|Default|GetMinutesPerDay) 6e+01)))

(fn GetSunandSky
  (Utilities|IsValid (Variables|Default|GetSun)
    (:Is%20Not%20Valid
      (bind _outactors (Actor|GetAllActorsOfClass "/Script/Engine.DirectionalLight"))
      (Variables|Default|SetSun (Utilities|Array|Get(acopy) _outactors))
      (Utilities|IsValid (Variables|Default|GetSky)
        (:Is%20Valid
          _)
        (:Is%20Not%20Valid
          (bind _outactors_2 (Actor|GetAllActorsOfClass "/Engine/EngineSky/BP_Sky_Sphere.BP_Sky_Sphere_C"))
          (Variables|Default|SetSky (Utilities|Array|Get(acopy) _outactors_2))))
      (Utilities|IsValid 0
        (:Is%20Not%20Valid
          (bind _outactors_3 (Actor|GetAllActorsOfClass "/Script/Engine.ExponentialHeightFog"))
          (Variables|Default|SetFog (Utilities|Array|Get(acopy) _outactors_3)))))))

(fn SetSunIntensity
  (Variables|Default|SetSunIntensity (Variables|/Script/Engine.LightComponentBase|GetIntensity (Variables|/Script/Engine.Light|GetLightComponent (Variables|Default|GetSun)))))

(fn SetElapsedTime
  (Variables|Default|SetElapsedTime (* (CallFunction|GetTimeasSeconds (Variables|Default|GetStartTime)) (/ (Variables|Default|GetSecondsPerDay) 8.64e+04))))

(fn GetTimeasSeconds
  (params (Time :type S%20Time%20Structure))
  (bind (_hours _minutes) (Utilities|Struct|BreakS_Time Time))
  (return (+ (* _hours 3600) (* _minutes 60))))

(fn UpdateElapsedTime
  (Variables|Default|SetElapsedTime (+ (Variables|Default|GetElapsedTime) (Utilities|Time|GetWorldDeltaSeconds))))

(fn UpdateSunPosition
  (Transformation|SetRelativeRotation (Variables|/Script/Engine.Light|GetLightComponent (Variables|Default|GetSun)) (Math|Rotator|MakeRotator 0.0 (+ (* (CallFunction|GetFractionOfDay) -3.6e+02) 9e+01) 4e+01) false false)
  (Default|UpdateSunDirection (Variables|Default|GetSky)))

(fn GetFractionOfDay
  (return (/ (Variables|Default|GetElapsedTime) (Variables|Default|GetSecondsPerDay))))

(fn UpdateCurrentTime
  (bind _output_get (Variables|Default|SetCurrentTime (CallFunction|DetermineCurrentTime)))
  (Default|SetTime (Variables|Default|GetHudReference) _output_get (Variables|Default|GetClockType)))

(fn DetermineCurrentTime
  (bind _returnvalue (CallFunction|GetFractionOfDay))
  (return (Utilities|Struct|MakeS_Time (Math|Float|Truncate (* (Math|Float|%(Float) _returnvalue 1.0) 24.0)) (Math|Float|Truncate (Math|Float|%(Float) (* _returnvalue 1.44e+03) 6e+01)))))

(fn FadeSun
  (bind _sun (Variables|Default|GetSun))
  (bind _lightcomponent (Variables|/Script/Engine.Light|GetLightComponent _sun))
  (Rendering|Components|Light|SetIntensity _lightcomponent (Math|Float|Clamp(Float) (+ (Variables|/Script/Engine.LightComponentBase|GetIntensity _lightcomponent) (* (Utilities|Time|GetWorldDeltaSeconds) (/ 24.0 (Variables|Default|GetSecondsPerDay)) (Variables|Default|GetSunIntensity) (select (CallFunction|DetermineNight) -1.0 1.0))) 0.0 (Variables|Default|GetSunIntensity))))

(fn DetermineNight
  (bind _currenttime (Variables|Default|GetCurrentTime))
  (return (or (< (.hours _currenttime) (Variables|Default|GetSunUpTime)) (>= (.hours _currenttime) (Variables|Default|GetSunDownTime)))))

(fn SetHUDRef
  (Utilities|IsValid (Variables|Default|GetHudReference)
    (:Is%20Not%20Valid
      (bind _asbp_principal (Utilities|Casting|CastToBP_Principal (Game|GetPlayerCharacter 0)))
      (Variables|Default|SetHudReference (Variables|/Game/Character/BP/Principal_Test/BP_Principal.BP_Principal_C|GetGameHUDRef _asbp_principal)))))
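; BP_Principal is the player character, handling movement, camera look and a switch between first- and third-person views.
; Axis inputs move the character relative to control yaw and feed controller yaw and pitch for looking.
; The POV action calls SwitchCamera, which toggles the active state of both the third-person and first-person cameras.
; On BeginPlay it creates the Widget_Time HUD, which displays the time, and adds it to the viewport.
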(event Collision|EventActorBeginOverlap
  (params (OtherActor :type Actor%20Object%20Reference)))

(event EventTick
  (params (DeltaSeconds :type Float%20%28single-precision%29)))

(event EventBeginPlay
  ;[1 1 1] affichage heure HUD
  (Utilities|FlowControl|Sequence
    (:then_0
      (bind _returnvalue (UserInterface|CreateWidget "/Game/Weather/Widget_Time.Widget_Time_C" (Game|GetPlayerController 0)))
      (bind _output_get (Variables|Default|SetGameHUDRef _returnvalue))
      (UserInterface|Viewport|AddtoViewport _output_get 0))))

(event Input|ActionEvents|InputActionPOV
  (params (Key :type Key%20Structure))
  ;[1 0 0.2137] Gestion Camera Perso
  (:Pressed
    (CallFunction|SwitchCamera)))

(event Input|AxisEvents|InputAxisMoveForward
  (params (AxisValue :type Float%20%28single-precision%29))
  ;[1 0.02467 0.2191] Avant/Arriere Personnage
  (Pawn|Input|AddMovementInput (Math|Vector|GetForwardVector (Math|Rotator|MakeRotator 0.0 0.0 (.Yaw (Math|Rotator|BreakRotator (Pawn|GetControlRotation :!class /Script/Engine.Pawn))))) AxisValue false))

(event Input|AxisEvents|InputAxisMoveRight
  (params (AxisValue :type Float%20%28single-precision%29))
  ;[1 0.02467 0.2191] Avant/Arriere Personnage
  (Pawn|Input|AddMovementInput (Math|Vector|GetRightVector (Math|Rotator|MakeRotator 0.0 0.0 (.Yaw (Math|Rotator|BreakRotator (Pawn|GetControlRotation :!class /Script/Engine.Pawn))))) AxisValue false))

(event Input|AxisEvents|InputAxisTurn
  (params (AxisValue :type Float%20%28single-precision%29))
  ;[1 0 0.2137] Gestion Camera Perso
  (Pawn|Input|AddControllerYawInput AxisValue))

(event Input|AxisEvents|InputAxisLockUp
  (params (AxisValue :type Float%20%28single-precision%29))
  ;[1 0 0.2137] Gestion Camera Perso
  (Pawn|Input|AddControllerPitchInput AxisValue))

(fn ConstructionScript)

(fn SwitchCamera
  (Components|Activation|ToggleActive (Variables|Default|GetCameratps)))